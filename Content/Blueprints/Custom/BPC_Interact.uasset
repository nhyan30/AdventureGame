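; Interaction component that lets its owning actor interact with objects in the world through the IA_Interact input action.
; When the input starts and CanInteract is true, it runs a short sphere trace on the Visibility channel from the owner's location, offset by the player camera's rotation.
; A successful trace calls InteractMessage on the hit actor, leaving the response to that actor.
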(event `EnhancedInput|/Game/Input/IA_Interact`
  (params (ActionValue :type Boolean) (ElapsedSeconds :type "Float (double-precision)") (TriggeredSeconds :type "Float (double-precision)") (InputAction :type "InputAction Object Reference" :default "/Game/Input/IA_Interact.IA_Interact"))
  (bind _returnvalue (`Actor.K2_GetActorLocation` (`self.GetOwner`)))
  (:`Started`
    (if (`self.Can Interact?`)
      (bind (_outhit _returnvalue_2) (`KismetSystemLibrary.SphereTraceSingle` _returnvalue (+ _returnvalue (* (`PlayerCameraManager.GetCameraRotation` (`GameplayStatics.GetPlayerCameraManager` 0)) 150.0)) 50.0 "TraceTypeQuery1"))
      (if _returnvalue_2
        (message `/Game/Blueprints/Custom/BBI_Interact.Interact` (`.HitActor` (`GameplayStatics.BreakHitResult` _outhit)))))))