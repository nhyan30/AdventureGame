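; BPC_Quest is a quest component that runs a single active quest at a time.
; StartQuest stores the quest, creates a WB_Quest widget, fills in its name and description and plays a sound, but only when none is active.
; CompleteQuest plays a sound and the widget's completion animation, then after a short delay removes the widget and clears the active flag.
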(event `Start Quest`
  (params (Quest :type "/Game/Blueprints/Custom/S_Quest Structure"))
  (bind (_current_quest_questname _current_quest_questdescription) (break `/Game/Blueprints/Custom/S_Quest` (`self.Current Quest`)))
  (if (not (`self.Active Quest?`))
    (set `self.Current Quest` Quest)
    (bind _returnvalue (`|CreateWidget` "/Game/Widgets/Custom/WB_Quest.WB_Quest_C"))
    (bind _output_get (set `self.Quest Widget` _returnvalue))
    (`UserWidget.AddToViewport` _output_get 0)
    (set `self.Active Quest?` true)
    (`TextBlock.SetText` (`/Game/Widgets/Custom/WB_Quest.ActiveQuestName` (`self.Quest Widget`)) (`KismetTextLibrary.Conv_NameToText` _current_quest_questname))
    (`TextBlock.SetText` (`/Game/Widgets/Custom/WB_Quest.ActiveQuestDescription` (`self.Quest Widget`)) (`KismetTextLibrary.Conv_NameToText` _current_quest_questdescription))
    (`GameplayStatics.PlaySound2D` "/Engine/EditorSounds/GamePreview/StartSimulate.StartSimulate" 1.0 1.0 0.0 null null)))

(event `Complete Quest`
  (bind _quest_widget (`self.Quest Widget`))
  (if (`self.Active Quest?`)
    (`GameplayStatics.PlaySound2D` "/Engine/EditorSounds/GamePreview/PossessPlayer.PossessPlayer" 1.0 1.0 0.0 null null)
    (`UserWidget.PlayAnimation` _quest_widget (`/Game/Widgets/Custom/WB_Quest.QuestCompletedNotification` _quest_widget) 0.0 1 "Forward" 1.0 false)
    (`KismetSystemLibrary.Delay` 2.0)
    (`Widget.RemoveFromParent` (`self.Quest Widget`))
    (set `self.Quest Widget` null)
    (set `self.Active Quest?` false)))